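; BP_Charater is a player character with side-scroller style movement, a score and hit points.
; Input moves it along the world Y axis and triggers jumps, while BeginPlay, overlap and Tick stay empty.
; SetScore adds to Score and prints the total.
; SetHp removes one HP per call and, once none remain, turns on mesh physics and collision for a ragdoll-style death and shows the Umg_end widget.
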(event `self.ReceiveBeginPlay`)

(event `InputAxis|MoveRight`
  (params (AxisValue :type "Float (single-precision)"))
  (`self.AddMovementInput` (0.0 -1.0 0.0) AxisValue))

(event `self.ReceiveActorBeginOverlap`
  (params (OtherActor :type "Actor Object Reference")))

(event `InputAction|Jump`
  (params (Key :type "Key Structure" :default "AnyKey"))
  (:`Pressed`
    (`self.Jump`)))

(event `self.ReceiveTick`
  (params (DeltaSeconds :type "Float (single-precision)")))

(fn `SetHp`
  (bind _mesh (`self.Mesh`))
  (bind _output_get (set `self.HP` (- (`self.HP`) 1)))
  (if (<= _output_get 0)
    (`PrimitiveComponent.SetSimulatePhysics` _mesh true)
    (`PrimitiveComponent.SetCollisionEnabled` _mesh "QueryAndPhysics")
    (bind _returnvalue (`|CreateWidget` "/Game/Blueprints/umg_end.umg_end_C"))
    (`UserWidget.AddToViewport` _returnvalue 0)))

(fn `SetScore`
  (params (Val :type Integer))
  (bind _output_get (set `self.Score` (+ Val (`self.Score`))))
  (`KismetSystemLibrary.PrintString` (`KismetStringLibrary.Conv_IntToString` _output_get)))

(fn `UserConstructionScript`)