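; Arrow projectile that explodes on hit and affects the player character's HP or score.
; ProjectileMovement drives the arrow mesh, and the actor destroys itself after a short lifetime if it hits nothing.
; A component hit spawns an explosion and destroys the arrow, then calls SetHp on a struck BP_Charater.
; Hitting any other actor calls SetScore on the player's pawn with a fixed value.
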(event `self.ReceiveBeginPlay`
  (`MovementComponent.SetUpdatedComponent` (`self.ProjectileMovement`) (`self.SM_Arrows`))
  (`KismetSystemLibrary.Delay` 3.5)
  (`self.K2_DestroyActor`))

(event `self.ReceiveActorBeginOverlap`
  (params (OtherActor :type "Actor Object Reference")))

(event `self.ReceiveTick`
  (params (DeltaSeconds :type "Float (single-precision)")))

(event `self.SM_Arrows.OnComponentHit`
  (params (OtherActor :type "Actor Object Reference") (OtherComp :type "PrimitiveComponent Object Reference") (NormalImpulse :type "Vector Structure") (Hit :type "HitResult Structure (by ref)"))
  (`GameplayStatics.SpawnEmitterAtLocation` "/Game/StarterContent/Particles/P_Explosion.P_Explosion" (`SceneComponent.K2_GetComponentLocation` (`self.SM_Arrows`)))
  (`self.K2_DestroyActor`)
  (bind _asbp_charater (cast `/Game/Blueprints/BP_Charater` OtherActor)
    (:`then`
      (`/Game/Blueprints/BP_Charater.SetHp` _asbp_charater))
    (:`CastFailed`
      (bind _asbp_charater_2 (cast `/Game/Blueprints/BP_Charater` (`GameplayStatics.GetPlayerPawn` 0)))
      (`/Game/Blueprints/BP_Charater.SetScore` _asbp_charater_2 50))))

(fn `UserConstructionScript`)